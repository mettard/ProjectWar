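; BP_CameraCharacter is a test camera pawn with an orthographic camera that zooms with the mouse wheel and shows the cursor.
; Wheel input steps a zoom multiplier clamped to configured bounds, and each Tick interpolates the ortho width toward step times multiplier.
; Disconnected leftover nodes would scale BP_TestVehicle widget draw sizes with the zoom level, but they never run.
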(event EventBeginPlay
  (Variables|/Script/Engine.PlayerController|SetbShowMouseCursor (Game|GetPlayerController 0) true)
  (Class|CameraComponent|SetOrthoWidth (Variables|Default|GetCamera) (* (Variables|Default|GetZoomStep) (Variables|Default|GetZoomMultiplier))))

(event EventTick
  (params (DeltaSeconds :type Float%20%28single-precision%29))
  (CallFunction|UpdateCameraZoom))

(event Input|MouseEvents|MouseWheelUp
  (params (Key :type Key%20Structure :default "None"))
  (bind _zoombounds (Variables|Default|GetZoomBounds))
  (:Pressed
    (Math|Float|DecrementFloat (Variables|Default|GetZoomMultiplier)
      (:%20%20
        (Variables|Default|SetZoomMultiplier (Math|Float|Clamp(Float) (Variables|Default|GetZoomMultiplier) (.x _zoombounds) (.y _zoombounds)))))))

(event Input|MouseEvents|MouseWheelDown
  (params (Key :type Key%20Structure :default "None"))
  (bind _zoombounds (Variables|Default|GetZoomBounds))
  (:Pressed
    (Math|Float|IncrementFloat (Variables|Default|GetZoomMultiplier)
      (:%20%20
        (Variables|Default|SetZoomMultiplier (Math|Float|Clamp(Float) (Variables|Default|GetZoomMultiplier) (.x _zoombounds) (.y _zoombounds)))))))

(fn ConstructionScript)

(fn UpdateCameraZoom
  (LocalVariables|SetTempCurrentZoom (Variables|/Script/Engine.CameraComponent|GetOrthoWidth (Variables|Default|GetCamera)))
  (Class|CameraComponent|SetOrthoWidth (Variables|Default|GetCamera) (Math|Interpolation|FInterpTo (LocalVariables|GetTempCurrentZoom) (* (Variables|Default|GetZoomStep) (Variables|Default|GetZoomMultiplier)) (Utilities|Time|GetWorldDeltaSeconds) 1e+01)))