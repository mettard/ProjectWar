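; Test AI controller base that uses an AI Perception component to react to actors it sees.
; On each perception update it checks every updated actor for sight and prints a placeholder "Hello" when one is sensed.
; The CanSenseActor helper maps a sense enum (Sight or Damage) to its sense class, then returns whether the first matching last-sensed stimulus was successfully sensed.
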(event OnPerceptionUpdated(AIPerception)
  (params (UpdatedActors :type Array%20of%20Actor%20Object%20References))
  (for _array_element UpdatedActors
    (bind _sensed (CallFunction|CanSenseActor _array_element "NewEnumerator1"))
    (if _sensed
      (Development|PrintString "Hello"))))

(event EventBeginPlay)

(event EventTick
  (params (DeltaSeconds :type Float%20%28single-precision%29)))

(fn ConstructionScript)

(fn CanSenseActor
  (params (Actor :type Actor%20Object%20Reference) (Sense :type NewUserDefinedEnum%20Enum :default "NewEnumerator0"))
  (bind _info (Class|AIPerceptionComponent|GetActorsPerception (Variables|Default|GetAIPerception) Actor))
  (for _array_element (.LastSensedStimuli (Utilities|Struct|BreakActorPerceptionBlueprintInfo _info))
    (bind _returnvalue (Class|AIPerceptionSystem|GetSenseClassforStimulus _array_element))
    (if (== _returnvalue (Utilities|Select :Index Sense :NewEnumerator0 0 :NewEnumerator1 "/Script/AIModule.AISense_Sight" :NewEnumerator2 "/Script/AIModule.AISense_Damage"))
      (return (.bSuccessfullySensed (Utilities|Struct|BreakAIStimulus _array_element))))))