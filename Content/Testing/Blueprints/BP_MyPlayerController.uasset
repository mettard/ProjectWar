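; Test player controller that zooms the camera and issues click-to-move orders to a vehicle.
; On BeginPlay it caches the BP_CameraCharacter, whose spring arm length the mouse wheel changes in fixed, unclamped steps.
; Right click runs a persistently drawn visibility trace from the camera toward an offset of the deprojected cursor position.
; A hit location goes to MovementToPoint on the BP_TestVehicle found by class lookup.
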(event EventBeginPlay
  ;[1 1 1] Camera
  ;;[1 1 1] Mapping
  (bind _asbp_camera_character (Utilities|Casting|CastToBP_CameraCharacter (Game|GetPlayerCharacter 0)))
  (Variables|Default|SetAs%20BP%20Camera%20Character _asbp_camera_character))

(event Input|MouseEvents|RightMouseButton
  (params (Key :type Key%20Structure :default "None"))
  ;[1 1 1] Camera
  (:Pressed
    (bind _returnvalue (Class|WidgetLayoutLibrary|GetMousePositiononViewport))
    (bind (_outhit _returnvalue_2) (Collision|LineTraceByChannel (Transformation|GetWorldLocation (Variables|/Game/Testing/Blueprints/BP_CameraCharacter.BP_CameraCharacter_C|GetCamera (Variables|Default|GetAs%20BP%20Camera%20Character))) (- (.WorldPosition (Class|GameplayStatics|DeprojectScreentoWorld (Game|GetPlayerController 0) _returnvalue)) 1e+05) "TraceTypeQuery1" false 0 "Persistent"))
    (if _returnvalue_2
      (bind _returnvalue_3 (Actor|GetActorOfClass "/Game/Testing/Blueprints/BP_TestVehicle.BP_TestVehicle_C"))
      (Default|MovementtoPoint _returnvalue_3 (.Location (Collision|BreakHitResult _outhit))))))

(event Input|MouseEvents|MouseWheelUp
  (params (Key :type Key%20Structure :default "None"))
  (bind _as_bp_camera_character (Variables|Default|GetAs%20BP%20Camera%20Character))
  (bind _springarm (Variables|/Game/Testing/Blueprints/BP_CameraCharacter.BP_CameraCharacter_C|GetSpringArm _as_bp_camera_character))
  ;[1 1 1] Camera
  ;;[1 1 1] Zoom in&out
  (:Pressed
    (Variables|/Script/Engine.SpringArmComponent|SetTargetArmLength _springarm (- (Variables|/Script/Engine.SpringArmComponent|GetTargetArmLength _springarm) 5e+02))))

(event Input|MouseEvents|MouseWheelDown
  (params (Key :type Key%20Structure :default "None"))
  (bind _as_bp_camera_character (Variables|Default|GetAs%20BP%20Camera%20Character))
  (bind _springarm (Variables|/Game/Testing/Blueprints/BP_CameraCharacter.BP_CameraCharacter_C|GetSpringArm _as_bp_camera_character))
  ;[1 1 1] Camera
  ;;[1 1 1] Zoom in&out
  (:Pressed
    (Variables|/Script/Engine.SpringArmComponent|SetTargetArmLength _springarm (- (Variables|/Script/Engine.SpringArmComponent|GetTargetArmLength _springarm) -5e+02))))

(fn ConstructionScript)