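; Player controller in a testing folder that drives a BP_CameraCharacter as a mouse-controlled camera with a visible cursor.
; BeginPlay caches the character and adds an Enhanced Input mapping context.
; MovingCamera (right mouse drag) offsets the character in world XY by the scaled viewport mouse delta each trigger, showing a grab-hand cursor meanwhile.
; Mouse wheel keys zoom by stepping the spring arm length, with no clamping.
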(event Input|EnhancedActionEvents|EnhancedInputActionMovingCamera
  (params (ActionValue :type Boolean) (ElapsedSeconds :type Float%20%28double-precision%29) (TriggeredSeconds :type Float%20%28double-precision%29) (InputAction :type Input%20Action%20Object%20Reference :default "/Game/Testing/Other/Mapping/MovingCamera.MovingCamera"))
  ;[1 1 1] Camera
  ;;[1 1 1] Movement character with right mouse button
  (:Triggered
    (bind _returnvalue (Class|WidgetLayoutLibrary|GetMousePositiononViewport))
    (bind _output_get (Variables|Default|SetCurrentMousePosition _returnvalue)))
  (:Started
    (bind _returnvalue_2 (Class|WidgetLayoutLibrary|GetMousePositiononViewport))
    (bind _output_get_2 (Variables|Default|SetStartMousePosition _returnvalue_2))))

(event Input|EnhancedActionEvents|EnhancedInputActionMovingCamera
  (params (ActionValue :type Boolean) (ElapsedSeconds :type Float%20%28double-precision%29) (TriggeredSeconds :type Float%20%28double-precision%29) (InputAction :type Input%20Action%20Object%20Reference :default "/Game/Testing/Other/Mapping/MovingCamera.MovingCamera"))
  ;[1 1 1] Camera
  ;;[1 1 1] Movement character with right mouse button
  (:Triggered
    (Variables|Default|SetCurrentMouseCursor "GrabHand")
    (Transformation|AddActorWorldOffset (Variables|Default|GetAs%20BP%20Camera%20Character) (Math|Vector|MakeVector (.X (Math|Vector2D|BreakVector2D (* (- (stale _output_get) (stale _output_get_2)) "(X=10.000000,Y=10.000000)"))) (.Y (Math|Vector2D|BreakVector2D (* (- (stale _output_get) (stale _output_get_2)) "(X=10.000000,Y=10.000000)"))) 0.0))
    (Variables|Default|SetStartMousePosition (Variables|Default|GetCurrentMousePosition)))
  (:Canceled
    (Variables|Default|SetCurrentMouseCursor "Default" :!label _label))
  (:Completed
    (goto _label)))

(event EventBeginPlay
  ;[1 1 1] Camera
  ;;[1 1 1] Mapping
  (bind _asbp_camera_character (Utilities|Casting|CastToBP_CameraCharacter (Game|GetPlayerCharacter 0)))
  (Variables|Default|SetAs%20BP%20Camera%20Character _asbp_camera_character)
  (Input|AddMappingContext (PlayerController|LocalPlayerSubsystems|GetEnhancedInputLocalPlayerSubsystem (Game|GetPlayerController 0)) "/Game/Testing/Other/Mapping/NewInputMappingContext.NewInputMappingContext" 0 "(bIgnoreAllPressedKeysUntilRelease=True,bForceImmediately=False,bNotifyUserSettings=False)")
  ;;[1 1 1] Mouse Cursor
  (Variables|/Script/Engine.PlayerController|SetbShowMouseCursor (Game|GetPlayerController (Variables|/Script/Engine.Pawn|GetPlayerState (Game|GetPlayerCharacter 0))) true))

(event Input|MouseEvents|MouseWheelUp
  (params (Key :type Key%20Structure :default "None"))
  (bind _as_bp_camera_character (Variables|Default|GetAs%20BP%20Camera%20Character))
  (bind _springarm (Variables|/Game/Testing/Sprites/BP_CameraCharacter.BP_CameraCharacter_C|GetSpringArm _as_bp_camera_character))
  ;[1 1 1] Camera
  ;;[1 1 1] Zoom in&out
  (:Pressed
    (Variables|/Script/Engine.SpringArmComponent|SetTargetArmLength _springarm (- (Variables|/Script/Engine.SpringArmComponent|GetTargetArmLength _springarm) 5e+02))))

(event Input|MouseEvents|MouseWheelDown
  (params (Key :type Key%20Structure :default "None"))
  (bind _as_bp_camera_character (Variables|Default|GetAs%20BP%20Camera%20Character))
  (bind _springarm (Variables|/Game/Testing/Sprites/BP_CameraCharacter.BP_CameraCharacter_C|GetSpringArm _as_bp_camera_character))
  ;[1 1 1] Camera
  ;;[1 1 1] Zoom in&out
  (:Pressed
    (Variables|/Script/Engine.SpringArmComponent|SetTargetArmLength _springarm (- (Variables|/Script/Engine.SpringArmComponent|GetTargetArmLength _springarm) -5e+02))))

(fn ConstructionScript)