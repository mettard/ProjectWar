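; BP_CameraCharacter is a test camera pawn with mouse-driven panning and zoom.
; Tick caches the viewport mouse position, and MovingCamera sets the actor's X/Y location directly from its swapped-axis offset to the right-click start point, rather than adding to the current location.
; The right button also toggles a Hold flag, read only by an empty Drag event.
; The mouse wheel steps the SpringArm length without clamping.
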(event Custom|Drag
  ;[1 1 1] Camera
  ;;[1 1 1] Movement character with right mouse button
  (if (Variables|Default|GetHold)
    _))

(event Input|EnhancedActionEvents|EnhancedInputActionMovingCamera
  (params (ActionValue :type Boolean) (ElapsedSeconds :type Float%20%28double-precision%29) (TriggeredSeconds :type Float%20%28double-precision%29) (InputAction :type Input%20Action%20Object%20Reference :default "/Game/Testing/Other/Mapping/MovingCamera.MovingCamera"))
  (:Triggered
    ;[1 1 1] Camera
    ;;[1 1 1] Movement character with right mouse button
    (Transformation|SetActorLocation (Math|Vector|MakeVector (.Y (Math|Vector2D|BreakVector2D (- (stale EventTick _output_get) (stale Input|MouseEvents|RightMouseButton _output_get)))) (.X (Math|Vector2D|BreakVector2D (- (stale EventTick _output_get) (stale Input|MouseEvents|RightMouseButton _output_get)))) 0.0) false false)))

(event EventTick
  (params (DeltaSeconds :type Float%20%28single-precision%29))
  ;[1 1 1] Camera
  ;;[1 1 1] Movement character with right mouse button
  (bind _returnvalue (Class|WidgetLayoutLibrary|GetMousePositiononViewport))
  (bind _output_get (Variables|Default|SetCurrentMousePosition _returnvalue)))

(event Input|MouseEvents|RightMouseButton
  (params (Key :type Key%20Structure :default "None"))
  ;[1 1 1] Camera
  ;;[1 1 1] Movement character with right mouse button
  (:Pressed
    (bind _returnvalue (Class|WidgetLayoutLibrary|GetMousePositiononViewport))
    (bind _output_get (Variables|Default|SetStartMousePosition _returnvalue))))

(event Input|MouseEvents|RightMouseButton
  (params (Key :type Key%20Structure :default "None"))
  (:Pressed
    (if (Game|Player|IsInputKeyDown (Game|GetPlayerController 0) Key)
      (Variables|Default|SetHold true)))
  (:Released
    (Variables|Default|SetHold false)))

(event Input|MouseEvents|MouseWheelUp
  (params (Key :type Key%20Structure :default "None"))
  ;[1 1 1] Camera
  ;;[1 1 1] Zoom in&out
  (:Pressed
    (Variables|/Script/Engine.SpringArmComponent|SetTargetArmLength (Variables|Default|GetSpringArm) (- (Variables|/Script/Engine.SpringArmComponent|GetTargetArmLength (Variables|Default|GetSpringArm)) 5e+02))))

(event Input|MouseEvents|MouseWheelDown
  (params (Key :type Key%20Structure :default "None"))
  ;[1 1 1] Camera
  ;;[1 1 1] Zoom in&out
  (:Pressed
    (Variables|/Script/Engine.SpringArmComponent|SetTargetArmLength (Variables|Default|GetSpringArm) (- (Variables|/Script/Engine.SpringArmComponent|GetTargetArmLength (Variables|Default|GetSpringArm)) -5e+02))))

(fn ConstructionScript)